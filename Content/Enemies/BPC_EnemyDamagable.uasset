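; BPC_EnemyDamagable is an enemy component that tracks health and handles damage and death.
; TakeDamage optionally plays a hit-react montage, subtracting damage only when the montage completes, or immediately when no reaction is requested.
; When health reaches zero or below, Death casts the owner to BP_ParentEnemy and unpossesses its controller if valid, with no destruction or death animation here.
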(event `TakeDamage`
  (params (`HitReact?` :type Boolean) (Damage :type "Float (double-precision)"))
  (if `HitReact?`
    (`|PlayMontage` null
      (:`OnCompleted`
        _)))
  (bind _output_get (set `self.Health` (- (`self.Health`) Damage)))
  (if (<= _output_get 0.0)
    (`self.Death`)))

(event `Death`
  (bind _asbp_parent_enemy (cast `/Game/Enemies/BP_ParentEnemy` (`self.GetOwner`)))
  (bind _returnvalue (`Pawn.GetController` _asbp_parent_enemy))
  (`/Engine/EditorBlueprintResources/StandardMacros.IsValid` _returnvalue
    (:`Is Valid`
      (`Controller.UnPossess` _returnvalue))))