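; BP_Enemy is an AI enemy that detects the player and turns into a physics ragdoll when it is unpossessed.
; AI perception writes the successfully sensed player into the TargetActor blackboard key, with nothing here clearing it when sensing is lost.
; On Unpossessed, it disables capsule collision responses and movement, enables mesh physics simulation, then destroys itself after a short delay.
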(event `self.ReceiveUnpossessed`
  (params (OldController :type "Controller Object Reference"))
  (`PrimitiveComponent.SetCollisionResponseToAllChannels` (`self.CapsuleComponent`) "ECR_Ignore")
  (`PrimitiveComponent.SetSimulatePhysics` (`self.Mesh`) true)
  (`CharacterMovementComponent.DisableMovement` (`self.CharacterMovement`))
  (`KismetSystemLibrary.Delay` 3.0)
  (`self.K2_DestroyActor`))

(event `self.AIPerception.OnTargetPerceptionUpdated`
  (params (Actor :type "Actor Object Reference") (Stimulus :type "AIStimulus Structure"))
  (if (== Actor (`GameplayStatics.GetPlayerCharacter` 0))
    (if (`.bSuccessfullySensed` (break `AIStimulus` Stimulus))
      (`/Engine/EditorBlueprintResources/StandardMacros.IsValid` Actor
        (:`Is Valid`
          (`BlackboardComponent.SetValueAsObject` (`AIBlueprintHelperLibrary.GetBlackboard` null) "TargetActor" Actor))))))

(fn `UserConstructionScript`)